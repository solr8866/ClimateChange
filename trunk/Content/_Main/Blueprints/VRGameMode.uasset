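; VR game mode that runs the narrated introduction when play begins and leads into the first choice.
; BeginPlay runs a linear Delay chain that fades the camera out and in, then plays two intro voice-over cues on one audio component, timed by each cue's duration.
; It then fades out again, plays the first choice line and calls the 02Choice1 dispatcher to hand off the next stage.
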(event `self.ReceiveBeginPlay`
  (bind _vo01_introduction_1_cue (`self.VO01_Introduction_1_Cue`))
  (bind _v_o_ (`self.V.O.`))
  (bind _v_o__2 (`self.V.O.`))
  (bind _vo01_introduction_2_cue (`self.VO01_Introduction_2_Cue`))
  (bind _vo02_choice_1_cue (`self.VO02_Choice_1_Cue`))
  (bind _v_o__3 (`self.V.O.`))
  ;[1 1 1] Introduction
  (`PlayerCameraManager.StartCameraFade` :`self` (`GameplayStatics.GetPlayerCameraManager` 0) :`FromAlpha` 0.0 :`ToAlpha` 1.0 :`Duration` (`self.FadeOutDuration`) :`bHoldWhenFinished` true)
  (`KismetSystemLibrary.Delay` 3.0)
  (`PlayerCameraManager.StartCameraFade` :`self` (`GameplayStatics.GetPlayerCameraManager` 0) :`FromAlpha` 1.0 :`ToAlpha` 0.0 :`Duration` (`self.FadeInDuration`) :`bHoldWhenFinished` true)
  (`KismetSystemLibrary.Delay` 2.0)
  (`AudioComponent.SetSound` _v_o_ _vo01_introduction_1_cue)
  (`AudioComponent.Play` _v_o_ 0.0)
  (`KismetSystemLibrary.Delay` (`SoundBase.Duration` _vo01_introduction_1_cue))
  (`AudioComponent.SetSound` _v_o__2 _vo01_introduction_2_cue)
  (`AudioComponent.Play` _v_o__2 0.0)
  (`KismetSystemLibrary.Delay` (`SoundBase.Duration` _vo01_introduction_2_cue))
  (`PlayerCameraManager.StartCameraFade` :`self` (`GameplayStatics.GetPlayerCameraManager` 0) :`ToAlpha` 1.0 :`Duration` 5.0 :`bHoldWhenFinished` true)
  (`KismetSystemLibrary.Delay` 2.0)
  (`AudioComponent.SetSound` _v_o__3 _vo02_choice_1_cue)
  (`AudioComponent.Play` _v_o__3 0.0)
  (`KismetSystemLibrary.Delay` (`SoundBase.Duration` _vo02_choice_1_cue))
  (`self.02_Choice_1`))

(fn `UserConstructionScript`)